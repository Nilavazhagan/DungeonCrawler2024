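; BP_KeyPickup is a spinning key pickup that grants its KeyID to whoever collects it.
; BeginPlay binds the Pickup component's OnPickup event, and Tick steadily yaws the scene root.
; On pickup, if the actor has a KeysInventoryComponent, the key ID is added to it, one of four random 2D pickup sounds plays, and the key destroys itself.
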(event Custom|KeyOnPickup
  (params (Actor :type Actor%20Object%20Reference))
  (bind _returnvalue (Actor|GetComponentbyClass Actor "/Script/DungeonCrawler2024.KeysInventoryComponent"))
  (Utilities|IsValid _returnvalue
    (:Is%20Valid
      (Class|KeysInventoryComponent|AddKeyID _returnvalue (Variables|Default|GetKeyID))
      (Audio|PlaySound2D (Utilities|Select :Index (Math|Random|RandomIntegerinRange 0 3) :Option%200 "/Game/Sound/KeyPickup/Key_PickUp.Key_PickUp" :Option%201 "/Game/Sound/KeyPickup/Key_PickUp_2.Key_PickUp_2" :Option%202 "/Game/Sound/KeyPickup/Key_PickUp_3.Key_PickUp_3" :Option%203 "/Game/Sound/KeyPickup/Key_PickUp_4.Key_PickUp_4") 5.0 1.0 0.0 0 0)
      (Actor|DestroyActor))))

(event EventBeginPlay
  (Variables|/Script/DungeonCrawler2024.PickupComponent|SetOnPickup (Variables|Default|GetPickup) (EventDispatchers|CreateEvent :!event Custom|KeyOnPickup)))

(event EventTick
  (params (DeltaSeconds :type Float%20%28single-precision%29))
  (Transformation|AddRelativeRotation (Variables|Default|GetDefaultSceneRoot) (Math|Rotator|MakeRotator 0.0 0.0 (* DeltaSeconds 3e+01)) false false))

(fn ConstructionScript)