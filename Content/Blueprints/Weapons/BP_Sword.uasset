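; BP_Sword is a melee weapon actor that plays a procedural swing and damages a target when attacked with.
; OnAttack restarts a timeline whose curves drive the WeaponPivot's relative location and rotation.
; An event track in that timeline times the hit, calling DamageComponent.DealDamageTo on the passed-in Target if valid, with no collision check.
; Debug strings print the target's name or flag an invalid target.
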(event EventBeginPlay
  (|CallParentFunction) ; This node is disabled and will not be called.\nDrag off pins to build functionality.
)

(event Collision|EventActorBeginOverlap
  (params (OtherActor :type Actor%20Object%20Reference))
  (|CallParentFunction OtherActor) ; This node is disabled and will not be called.\nDrag off pins to build functionality.
)

(event EventTick
  (params (DeltaSeconds :type Float%20%28single-precision%29))
  (|CallParentFunction DeltaSeconds) ; This node is disabled and will not be called.\nDrag off pins to build functionality.
)

(event EventOnAttack
  (params (Attacker :type Actor%20Object%20Reference) (Target :type Actor%20Object%20Reference))
  (bind (_direction _weaponlocation _weaponrotation) (Timeline|Timeline PlayFromStart)
    (:Update
      (Utilities|FlowControl|Sequence
        (:then_0
          (Transformation|SetRelativeLocation (Variables|Default|GetWeaponPivot) _weaponlocation false false))
        (:then_1
          (Transformation|SetRelativeRotation (Variables|Default|GetWeaponPivot) (Math|Rotator|MakeRotator (.X (Math|Vector|BreakVector _weaponrotation)) (.Y (Math|Vector|BreakVector _weaponrotation)) 0.0) false false))))
    (:DamageDealDamage
      (Utilities|IsValid Target
        (:Is%20Valid
          (Development|PrintString (Utilities|GetDisplayName Target))
          (Class|DamageComponent|DealDamageto (Variables|Default|GetDamageComponent) Target Attacker))
        (:Is%20Not%20Valid
          (Development|PrintString "Target Invalid!"))))))

(fn ConstructionScript
  (|CallParentFunction))