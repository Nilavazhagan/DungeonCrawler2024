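; BP_Weapon is a weapon actor that plays a swing animation and deals damage when told to attack.
; OnAttack starts the WeaponSwing timeline, which pitches the WeaponPivot and fires an event track at the damage moment.
; That event passes attacker and target to DamageComponent if the target is valid.
; Otherwise it clears the input block on a PlayerCharacter attacker; debug prints trace each step.
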(event EventBeginPlay)

(event Collision|EventActorBeginOverlap
  (params (OtherActor :type Actor%20Object%20Reference)))

(event EventTick
  (params (DeltaSeconds :type Float%20%28single-precision%29)))

(event EventOnAttack
  (params (Attacker :type Actor%20Object%20Reference) (Target :type Actor%20Object%20Reference))
  (Development|PrintText "BP_Weaon is attacking!")
  (bind _weaponrotation (Timeline|Weapon%20Swing PlayFromStart)
    (:Update
      (Transformation|SetRelativeRotation (Variables|Default|GetWeaponPivot) (Math|Rotator|MakeRotator 0.0 _weaponrotation 0.0) false false))
    (:DamageDealDamage
      (Utilities|IsValid Target
        (:Is%20Valid
          (Development|PrintString (Utilities|GetDisplayName Target))
          (Class|DamageComponent|DealDamageto (Variables|Default|GetDamageComponent) Target Attacker))
        (:Is%20Not%20Valid
          (Development|PrintString "Target Invalid!")
          (bind _asplayer_character (Utilities|Casting|CastToPlayerCharacter Attacker))
          (Class|PlayerCharacter|SetShouldBlockInput _asplayer_character false))))))

(fn ConstructionScript)