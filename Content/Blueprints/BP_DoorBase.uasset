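; Base door Blueprint that opens and closes when an actor interacts with it, optionally requiring a key.
; When locked, it checks the actor's KeysInventoryComponent for its KeyID, playing a lock sound if the key is missing.
; A timeline swings the door pivot forward or in reverse with sounds, then updates TileBlocking from the open state.
; Finished swings and missing-key attempts call TickIfTrue on the interacting PlayerCharacter.
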(event Custom|OpenOrCloseDoor
  ;[1 1 1] Open or close the door
  (if (Variables|Default|GetIsOpen)
    (Audio|Components|Audio|Play (Variables|Default|GetDoorCloseSound) 0.0)
    (Utilities|FlowControl|Sequence
      (:then_0
        (Variables|Default|SetIsOpen (not (Variables|Default|GetIsOpen)) :!label _label))
      (:then_1
        (bind _doorangle (Timeline|DoorOpen Reverse)
          (:Update
            (Transformation|SetRelativeRotation (Variables|Default|GetDoorPivot) (Math|Rotator|MakeRotator 0.0 0.0 _doorangle) false false))
          (:Finished
            (Variables|/Script/DungeonCrawler2024.TileBlockingComponent|SetbDoesBlockTile (Variables|Default|GetTileBlocking) (not (Variables|Default|GetIsOpen)))
            (bind _asplayer_character (Utilities|Casting|CastToPlayerCharacter (Variables|Default|GetDoer%20Actor)))
            (Class|PlayerCharacter|TickifTrue _asplayer_character true)))))
    (else
      (Audio|Components|Audio|Play (Variables|Default|GetDoorOpenSound) 0.0)
      (Utilities|FlowControl|Sequence
        (:then_0
          (goto _label))
        (:then_1
          (Timeline|DoorOpen Play))))))

(event EventOnInteract
  (params (DoerActor :type Actor%20Object%20Reference))
  (Variables|Default|SetDoer%20Actor DoerActor)
  (Development|PrintText "INTERACTING!")
  (if (Variables|Default|GetIsLocked)
    ;[1 1 1] If locked, check for the key in player's inventory, then unlock and open if they have it
    (Utilities|IsValid (Actor|GetComponentbyClass (Variables|Default|GetDoer%20Actor) "/Script/DungeonCrawler2024.KeysInventoryComponent")
      (:Is%20Valid
        (bind _returnvalue (Class|KeysInventoryComponent|GetHasKeyID (Actor|GetComponentbyClass (Variables|Default|GetDoer%20Actor) "/Script/DungeonCrawler2024.KeysInventoryComponent") (Variables|Default|GetKeyID)))
        (if _returnvalue
          (Audio|PlaySound2D "/Game/Sound/LockRattles/Lock_Rattle_3.Lock_Rattle_3" 1.0 1.0 0.0 0 0 false)
          (CallFunction|OpenorCloseDoor)
          (else
            (Audio|Components|Audio|Play (Variables|Default|GetDoorLockSound) 0.0)
            (bind _asplayer_character (Utilities|Casting|CastToPlayerCharacter (Variables|Default|GetDoer%20Actor)))
            (Class|PlayerCharacter|TickifTrue _asplayer_character true)))))
    (else
      (CallFunction|OpenorCloseDoor))))

(event Collision|EventActorBeginOverlap
  (params (OtherActor :type Actor%20Object%20Reference)))

(event EventTick
  (params (DeltaSeconds :type Float%20%28single-precision%29)))

(fn ConstructionScript)