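; BP_Door is an interactable door that swings open and closed and controls whether its tile is blocked.
; On interact it prints a debug message, then, unless locked, toggles IsOpen and plays or reverses the DoorOpen timeline.
; The timeline drives the yaw of DoorPivot and, when finished, sets the TileBlocking component to block only while the door is closed.
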(event EventOnInteract
  (params (DoerActor :type Actor%20Object%20Reference))
  (Development|PrintText "INTERACTING!")
  (if (not (Variables|Default|GetIsLocked))
    (if (Variables|Default|GetIsOpen)
      (Utilities|FlowControl|Sequence
        (:then_0
          (Variables|Default|SetIsOpen (not (Variables|Default|GetIsOpen)) :!label _label))
        (:then_1
          (bind _doorangle (Timeline|DoorOpen Reverse)
            (:Update
              (Transformation|SetRelativeRotation (Variables|Default|GetDoorPivot) (Math|Rotator|MakeRotator 0.0 0.0 _doorangle) false false))
            (:Finished
              (Variables|/Script/DungeonCrawler2024.TileBlockingComponent|SetbDoesBlockTile (Variables|Default|GetTileBlocking) (not (Variables|Default|GetIsOpen)))))))
      (else
        (Utilities|FlowControl|Sequence
          (:then_0
            (goto _label))
          (:then_1
            (Timeline|DoorOpen Play)))))))

(event Collision|EventActorBeginOverlap
  (params (OtherActor :type Actor%20Object%20Reference)))

(event EventTick
  (params (DeltaSeconds :type Float%20%28single-precision%29)))

(fn ConstructionScript)